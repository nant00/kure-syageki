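; BP_Ldestroy is a moving shooting target that breaks apart when hit by a FirstPersonProjectile and awards points.
; On BeginPlay it adds a Scorewiget to the viewport and plays a timeline that offsets it along local Y, recreating a dynamic wall material on every update.
; A projectile hit applies radius damage to the ShapeSphereDM destructible, increments the player character's Point, then destroys the actor after a short delay.
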(event `self.ReceiveBeginPlay`
  ;[1 1 1] UI表示
  (bind _returnvalue (`|CreateWidget` "/Game/FirstPersonBP/Blueprints/scorewiget.scorewiget_C"))
  (`UserWidget.AddToViewport` _returnvalue 0)
  ;[1 1 1] targetの動く挙動
  (bind (_direction `_新規track_0`) (`Timeline|タイムライン_0`)
    (:`Update`
      (`self.K2_AddActorLocalOffset` (`KismetMathLibrary.MakeVector` 0.0 `_新規track_0`))
      (bind _returnvalue_2 (`PrimitiveComponent.CreateDynamicMaterialInstance` (`self.Shape_Sphere_DM`) 0 "/Game/FirstPerson/shape/M_Basic_Wall.M_Basic_Wall" "None"))
      (set `self.MID` _returnvalue_2))))

(event `self.ReceiveHit`
  (params (MyComp :type "PrimitiveComponent Object Reference") (Other :type "Actor Object Reference") (OtherComp :type "PrimitiveComponent Object Reference") (bSelfMoved :type Boolean) (HitLocation :type "Vector Structure") (HitNormal :type "Vector Structure") (NormalImpulse :type "Vector Structure") (Hit :type "HitResult Structure (by ref)"))
  (bind _shape_sphere_dm (`self.Shape_Sphere_DM`))
  ;[1 1 1] 弾との当たり判定
  (cast `/Game/FirstPersonBP/Blueprints/FirstPersonProjectile` Other)
  (`DestructibleComponent.ApplyRadiusDamage` _shape_sphere_dm 100.0 (`SceneComponent.K2_GetComponentLocation` _shape_sphere_dm) 100.0 1000.0 false)
  ;[1 1 1] スコア加算
  (bind _asfirst_person_character (cast `/Game/FirstPersonBP/Blueprints/FirstPersonCharacter` (`GameplayStatics.GetPlayerCharacter` 0)))
  (set `/Game/FirstPersonBP/Blueprints/FirstPersonCharacter.point` (+ (`/Game/FirstPersonBP/Blueprints/FirstPersonCharacter.point` _asfirst_person_character) 1) _asfirst_person_character)
  ;[1 1 1] 破壊したオブジェトの消去
  (`KismetSystemLibrary.Delay` 2.0)
  (`self.K2_DestroyActor`))

(fn `UserConstructionScript`)